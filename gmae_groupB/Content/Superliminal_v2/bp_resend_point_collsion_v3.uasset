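; Trigger volume that teleports the FPS_Superliminal_v3 player to a resend spawn point when they overlap its Box.
; On BeginPlay it caches the destination by using ResendPoint as an index into all BP_resend_spawn_location_v2 actors, so pairing depends on that array's order.
; Overlap sets CanResend false before the move and again after a short delay; the branch that would check the flag is unconnected.
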(event OnComponentBeginOverlap(Box)
  (params (OverlappedComponent :type Primitive%20Component%20Object%20Reference) (OtherActor :type Actor%20Object%20Reference) (OtherComp :type Primitive%20Component%20Object%20Reference) (OtherBodyIndex :type Integer) (bFromSweep :type Boolean) (SweepResult :type Hit%20Result%20Structure%20%28by%20ref%29))
  (bind _asfps_superliminal_v_3 (Utilities|Casting|CastToFPS_Superliminal_v3 OtherActor))
  (Variables|/Game/Superliminal/FPS_Superliminal_v3.FPS_Superliminal_v3_C|Setcan%20resend? _asfps_superliminal_v_3 false)
  (Transformation|SetActorLocationAndRotation _asfps_superliminal_v_3 (Transformation|GetActorLocation (Variables|Default|Getspawn%20location)))
  (Utilities|FlowControl|Delay 0.1)
  (Variables|/Game/Superliminal/FPS_Superliminal_v3.FPS_Superliminal_v3_C|Setcan%20resend? _asfps_superliminal_v_3 false))

(event EventBeginPlay
  (bind _outactors (Actor|GetAllActorsOfClass "/Game/Superliminal_v2/BP_resend_spawn_location_v2.BP_resend_spawn_location_v2_C"))
  (Variables|Default|Setspawn%20location (Utilities|Array|Get(acopy) _outactors (Variables|Default|Getresend%20point))))

(event Collision|EventActorBeginOverlap
  (params (OtherActor :type Actor%20Object%20Reference)))

(event EventTick
  (params (DeltaSeconds :type Float%20%28single-precision%29)))

(fn ConstructionScript)