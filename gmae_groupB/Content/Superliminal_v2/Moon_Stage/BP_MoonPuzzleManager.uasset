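; Puzzle manager for the Moon Stage that runs a one-time completion event once the fixed-puzzle count reaches the required total.
; CheckPuzzleProgress plays a sound, stops the BGM actor, disables player input and, after a short delay, plays the door-opening Level Sequence.
; A fixed timer then calls MoveAgain, which restores input, reveals BP_WalkRoud, destroys tagged wall actors and restarts the BGM.
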(event Custom|CheckPuzzleProgress
  (if (>= (Variables|Default|GetMoon_CurrentPuzzleFixed) (Variables|Default|GetMoon_TotalPuzzleNeed))
    (Utilities|FlowControl|DoOnce false
      (:Completed
        (Audio|PlaySoundatLocation "/Game/Superliminal_v2/Moon_Stage/soundreality-button-4-214382.soundreality-button-4-214382" "0, 0, 0" "0, 0, 0" 1.0 1.0 0.0 0 0 0 0)
        (bind _returnvalue (Actor|GetActorOfClass "/Game/Blueprints/BP_BGM.BP_BGM_C"))
        (Default|Stop _returnvalue)
        (Input|DisableInput (Game|GetPlayerCharacter 0) (Game|GetPlayerController 0))
        (Utilities|FlowControl|Sequence
          (:then_0
            (Utilities|FlowControl|Delay 1.0)
            (bind _outactor (Sequencer|Player|CreateLevelSequencePlayer "/Game/Superliminal_v2/adeline_v2/openDoor_LevelSequence.openDoor_LevelSequence"))
            (Sequencer|Player|Play (Variables|/Script/LevelSequence.LevelSequenceActor|GetSequencePlayer _outactor) :!class /Script/MovieScene.MovieSceneSequencePlayer))
          (:then_1
            (Utilities|Time|SetTimerbyEvent (delegate Custom|MoveAgain) 10.6)))))))

(event Custom|MoveAgain
  (Input|EnableInput (Game|GetPlayerCharacter 0) (Game|GetPlayerController 0))
  (bind _returnvalue (Actor|GetActorOfClass "/Game/Superliminal_v2/Moon_Stage/BP_WalkRoud.BP_WalkRoud_C"))
  (Rendering|SetActorHiddenInGame _returnvalue false)
  (bind _outactors (Actor|GetAllActorswithTag "MoonStage_Wall"))
  (Actor|DestroyActor _outactors)
  (bind _returnvalue_2 (Actor|GetActorOfClass "/Game/Blueprints/BP_BGM.BP_BGM_C"))
  (Default|Play _returnvalue_2))

(fn ConstructionScript)