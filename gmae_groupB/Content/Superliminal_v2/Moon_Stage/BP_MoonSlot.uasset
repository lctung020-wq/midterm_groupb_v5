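; BP_MoonSlot is a puzzle slot in the Moon stage that accepts the BP_PuzzleSelf piece whose PuzzleID matches its MoonPuzzleID.
; On a matching box overlap it makes the player drop the piece, snaps and destroys it, shows its Fire component, and detaches its mesh with physics and collision off.
; It then increments BP_MoonPuzzleManager's fixed count and triggers a progress check.
; A mismatched piece hides the Fire, which also starts hidden.
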(event OnComponentBeginOverlap(BoxCollision)
  (params (OverlappedComponent :type Primitive%20Component%20Object%20Reference) (OtherActor :type Actor%20Object%20Reference) (OtherComp :type Primitive%20Component%20Object%20Reference) (OtherBodyIndex :type Integer) (bFromSweep :type Boolean) (SweepResult :type Hit%20Result%20Structure%20%28by%20ref%29))
  (bind _staticmesh (Variables|Default|GetStaticMesh))
  (bind _asbp_puzzle_self (Utilities|Casting|CastToBP_PuzzleSelf OtherActor))
  (if (== (Variables|/Game/Puzzle/BP_PuzzleSelf.BP_PuzzleSelf_C|GetPuzzleID _asbp_puzzle_self) (Variables|Default|GetMoon_PuzzleID))
    (bind _asfps_superliminal_v_3 (Utilities|Casting|CastToFPS_Superliminal_v3 (Game|GetPlayerCharacter 0)))
    (Default|DropPuzzle _asfps_superliminal_v_3)
    (Transformation|SetActorLocationAndRotation _asbp_puzzle_self (Transformation|GetActorLocation) (Transformation|GetActorRotation))
    (Rendering|SetVisibility (Variables|Default|GetFire) true false)
    (Actor|DestroyActor _asbp_puzzle_self)
    (Transformation|DetachFromComponent (Variables|Default|GetStaticMesh) "KeepWorld" "KeepWorld" "KeepWorld" true)
    (Physics|SetSimulatePhysics _staticmesh false)
    (Collision|SetCollisionEnabled _staticmesh "NoCollision")
    (bind _returnvalue (Actor|GetActorOfClass "/Game/Superliminal_v2/Moon_Stage/BP_MoonPuzzleManager.BP_MoonPuzzleManager_C"))
    (Variables|/Game/Superliminal_v2/Moon_Stage/BP_MoonPuzzleManager.BP_MoonPuzzleManager_C|SetMoon_CurrentPuzzleFixed _returnvalue (+ (Variables|/Game/Superliminal_v2/Moon_Stage/BP_MoonPuzzleManager.BP_MoonPuzzleManager_C|GetMoon_CurrentPuzzleFixed _returnvalue) 1))
    (Default|CheckPuzzleProgress _returnvalue)
    (else
      (Rendering|SetVisibility (Variables|Default|GetFire) false false))))

(event EventBeginPlay
  (Rendering|SetVisibility (Variables|Default|GetFire) false false))

(fn ConstructionScript
  (|CallParentFunction))