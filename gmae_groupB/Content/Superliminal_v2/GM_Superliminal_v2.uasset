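; Game mode for Superliminal v2 that picks where the player spawns, based on a tag held in the game instance.
; It overrides ChoosePlayerStart to read TargetPlayerTag from MyPortalGI and return the first PlayerStart with that tag.
; When the tag is None, it falls back to the first PlayerStart found in the level.
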(event EventBeginPlay)

(event EventTick
  (params (DeltaSeconds :type Float%20%28single-precision%29)))

(fn ConstructionScript)

(fn ChoosePlayerStart
  (params (Player :type Controller%20Object%20Reference))
  (bind _asmy_portal_gi (Utilities|Casting|CastToMyPortalGI (Game|GetGameInstance)))
  (if (!= (Variables|/Game/Superliminal_v2/adeline_v2/MyPortalGI.MyPortalGI_C|GetTargetPlayerTag _asmy_portal_gi) "")
    (bind _outactors (Actor|GetAllActorsOfClasswithTag "/Script/Engine.PlayerStart" (Variables|/Game/Superliminal_v2/adeline_v2/MyPortalGI.MyPortalGI_C|GetTargetPlayerTag _asmy_portal_gi)))
    (return (Utilities|Array|Get(acopy) _outactors))
    (else
      (bind _outactors_2 (Actor|GetAllActorsOfClass "/Script/Engine.PlayerStart"))
      (return (Utilities|Array|Get(acopy) _outactors_2)))))