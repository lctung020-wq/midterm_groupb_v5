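; A memory pickup actor that spins its static mesh every tick and opens a paged reading widget when collected.
; Capsule overlap by the Superliminal FPS character creates the widget with the cover texture, page count and page images, adds it to the viewport, then destroys the pickup.
; BeginPlay applies the configured mesh and caches an indexed MemoryPickup2 widget reference, which the graph never uses afterwards.
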(event OnComponentBeginOverlap(Capsule)
  (params (OverlappedComponent :type Primitive%20Component%20Object%20Reference) (OtherActor :type Actor%20Object%20Reference) (OtherComp :type Primitive%20Component%20Object%20Reference) (OtherBodyIndex :type Integer) (bFromSweep :type Boolean) (SweepResult :type Hit%20Result%20Structure%20%28by%20ref%29))
  (Utilities|Casting|CastToFPS_Superliminal_v3 OtherActor)
  (Variables|Default|Setis%20reading? true)
  (if (Variables|Default|Getis%20reading?)
    (bind _returnvalue (UserInterface|CreateWidget "/Game/Superliminal_v2/adeline_v2/memory_bp/memPickup_haveP_UWG1.memPickup_haveP_UWG1_C" (Game|GetPlayerController 0) (Variables|Default|GetCover%20Texture) (Variables|Default|GetPage%20Max) (Variables|Default|Getpage_image_ref)))
    (UserInterface|Viewport|AddtoViewport _returnvalue 0)
    (Actor|DestroyActor self)))

(event Collision|EventActorBeginOverlap
  (params (OtherActor :type Actor%20Object%20Reference)))

(event EventTick
  (params (DeltaSeconds :type Float%20%28single-precision%29))
  (Transformation|AddLocalRotation (Variables|Default|GetStaticMesh) (Variables|Default|GetDelta%20Rotation) false false))

(event EventBeginPlay
  (Components|StaticMesh|SetStaticMesh (Variables|Default|GetStaticMesh) (Variables|Default|GetNew%20Mesh))
  (bind _foundwidgets (Widget|GetAllWidgetsOfClass "/Game/Superliminal_v2/adeline_v2/memory_bp/memoryPickup2_UWG.memoryPickup2_UWG_C" true))
  (Variables|Default|Setwhich_UMG (Utilities|Array|Get(acopy) _foundwidgets (Variables|Default|GetNO_of_UMG))))

(fn ConstructionScript)