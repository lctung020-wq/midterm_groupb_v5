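; BP_PuzzleSlot is a puzzle slot that accepts a BP_PuzzleSelf piece with a matching PuzzleID.
; When a matching piece overlaps its box, it makes the FPS_Superliminal_v3 player drop it, snaps it to the slot, then destroys it.
; The slot's TargetPoints takes the Shading material, detaches and loses physics and collision, standing in for the piece.
; It then increments BP_PuzzleManager's fixed count and triggers a progress check.
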(event OnComponentBeginOverlap(BoxCollision)
  (params (OverlappedComponent :type Primitive%20Component%20Object%20Reference) (OtherActor :type Actor%20Object%20Reference) (OtherComp :type Primitive%20Component%20Object%20Reference) (OtherBodyIndex :type Integer) (bFromSweep :type Boolean) (SweepResult :type Hit%20Result%20Structure%20%28by%20ref%29))
  (bind _target_points (Variables|Default|GetTarget%20Points))
  (bind _asbp_puzzle_self (Utilities|Casting|CastToBP_PuzzleSelf OtherActor))
  (if (== (Variables|/Game/Puzzle/BP_PuzzleSelf.BP_PuzzleSelf_C|GetPuzzleID _asbp_puzzle_self) (Variables|Default|GetPuzzleID))
    (bind _asfps_superliminal_v_3 (Utilities|Casting|CastToFPS_Superliminal_v3 (Game|GetPlayerCharacter 0)))
    (Default|DropPuzzle _asfps_superliminal_v_3)
    (Transformation|SetActorLocationAndRotation _asbp_puzzle_self (Transformation|GetActorLocation) (Transformation|GetActorRotation))
    (Rendering|Material|SetMaterial (Variables|Default|GetTarget%20Points) 0 (Variables|Default|GetShading))
    (Actor|DestroyActor _asbp_puzzle_self)
    (Transformation|DetachFromComponent (Variables|Default|GetTarget%20Points) "KeepWorld" "KeepWorld" "KeepWorld" true)
    (Physics|SetSimulatePhysics _target_points false)
    (Collision|SetCollisionEnabled _target_points "NoCollision")
    (bind _returnvalue (Actor|GetActorOfClass "/Game/Puzzle/BP_PuzzleManager.BP_PuzzleManager_C"))
    (Variables|/Game/Puzzle/BP_PuzzleManager.BP_PuzzleManager_C|SetCurrentPuzzleFixed _returnvalue (+ (Variables|/Game/Puzzle/BP_PuzzleManager.BP_PuzzleManager_C|GetCurrentPuzzleFixed _returnvalue) 1))
    (Default|CheckPuzzleProgress _returnvalue)))

(fn ConstructionScript)